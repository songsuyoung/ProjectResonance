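; BP_NPCTest is a debug Blueprint for testing NPC stat changes by keyboard.
; A RegisterNPC event stores a reference to the NPC character to be tested.
; Pressing Q lowers that NPC's Stamina and W lowers its Mood by a fixed step, reading and writing values through its BaseStatComponent.
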(event `RegisterNPC`
  (params (NPCCharacter :type "/Game/Blueprints/NPC/BP_NPC Object Reference"))
  (set `self.NPCCharacter` NPCCharacter))

(event `Key|Q`
  (params (Key :type "Key Structure"))
  (bind _basestatcomponent (`RBaseCharacter.BaseStatComponent` (`self.NPCCharacter`)))
  (:`Pressed`
    (bind _returnvalue (`RBaseStatComponent.GetStatValue` _basestatcomponent "Stamina"))
    (`RBaseStatComponent.UpdateStat` _basestatcomponent "Stamina" (- _returnvalue 10.0))))

(event `Key|W`
  (params (Key :type "Key Structure"))
  (bind _basestatcomponent (`RBaseCharacter.BaseStatComponent` (`self.NPCCharacter`)))
  (:`Pressed`
    (bind _returnvalue (`RBaseStatComponent.GetStatValue` _basestatcomponent "Mood"))
    (`RBaseStatComponent.UpdateStat` _basestatcomponent "Mood" (- _returnvalue 10.0))))

(fn `UserConstructionScript`)